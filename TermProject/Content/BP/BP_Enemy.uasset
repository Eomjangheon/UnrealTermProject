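; BP_Enemy is an enemy that plays a death and dissolve effect when it takes any damage, with no health check.
; AnyDamage plays the Mutant_dying animation once and creates a dynamic material instance on the mesh's first material slot.
; A Timeline then lowers an "Amount" parameter on both that material and the Dissolve effect component, keeping the two in step.
; The actor is not destroyed afterwards.
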(event `self.ReceiveAnyDamage`
  (params (Damage :type "Float (single-precision)") (DamageType :type "DamageType Object Reference") (InstigatedBy :type "Controller Object Reference") (DamageCauser :type "Actor Object Reference"))
  (bind _mesh (`self.Mesh`))
  (`SkeletalMeshComponent.PlayAnimation` (`self.Mesh`) "/Game/Animation/Enemy/mutant_dying.mutant_dying" false)
  (bind _returnvalue (`PrimitiveComponent.CreateDynamicMaterialInstance` _mesh 0 (`PrimitiveComponent.GetMaterial` _mesh 0) "None"))
  (bind (_direction _newtrack_0) (`Timeline|Timeline` :!via `PlayFromStart`)
    (:`Update`
      (`MaterialInstanceDynamic.SetScalarParameterValue` _returnvalue "Amount" (`KismetMathLibrary.Lerp` 1.0 0.0 _newtrack_0))
      (`NiagaraComponent.SetVariableFloat` (`self.Dissolve`) "Amount" (`KismetMathLibrary.Lerp` 1.0 -0.1 _newtrack_0)))))

(fn `UserConstructionScript`)