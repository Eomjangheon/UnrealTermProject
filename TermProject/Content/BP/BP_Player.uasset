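; Player character Blueprint for sword combat, gating jump, double jump, attack and dodge through a SwordState enum.
; Combo input plays three-step ground or air montage chains by AttackCount, with launches lunging the ground finisher and lifting every air hit.
; Input during attacks is buffered in SaveAttack until ComboAttackSave continues the chain; ResetCombo clears it.
; Dodge picks one of four montages by input angle, launches that way, and can cancel ground attacks.
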(event `self.ReceiveTick`
  (params (DeltaSeconds :type "Float (single-precision)")))

(event `self.ReceiveBeginPlay`)

(event `JumpEvent`
  ;[1 1 1] Jump/DoubleJump
  (switch `/Game/Enum/EnumSwordState` (`self.SwordState`)
    (:`NewEnumerator0`
      (set `self.SwordState` "NewEnumerator2" :!label _label)
      (`self.Jump`))
    (:`NewEnumerator1`
      (goto _label))
    (:`NewEnumerator2`
      (set `self.SwordState` "NewEnumerator3")
      (`self.LaunchCharacter` (`KismetMathLibrary.MakeVector` 0.0 0.0 (`CharacterMovementComponent.JumpZVelocity` (`self.CharacterMovement`))) false true))))

(event `self.OnLanded`
  (params (Hit :type "HitResult Structure (by ref)"))
  ;[1 1 1] Landing
  (switch `/Game/Enum/EnumSwordState` (`self.SwordState`)
    (:`NewEnumerator2`
      _)
    (:`NewEnumerator3`
      _)
    (:`NewEnumerator4`
      _))
  (set `self.SwordState` "NewEnumerator0"))

(event `Combo3Input`
  (bind _attackcount (`self.AttackCount`))
  ;[1 1 1] SetCombo
  (switch `/Game/Enum/EnumSwordState` (`self.SwordState`)
    (:`NewEnumerator0`
      (set `self.SwordState` "NewEnumerator6" :!label _label_2)
      ;[1 1 1] GroundAttack
      (switch `int` _attackcount :!label _label_3
        (:`0`
          (set `self.AttackCount` 1)
          (`self.PlayAnimMontage` "/Game/Animation/Combo3_1.Combo3_1"))
        (:`1`
          (set `self.AttackCount` 2)
          (`self.PlayAnimMontage` "/Game/Animation/Combo3_2.Combo3_2"))
        (:`2`
          (set `self.AttackCount` 0)
          (`self.PlayAnimMontage` "/Game/Animation/Combo3_3.Combo3_3")
          (`self.LaunchCharacter` (* (`self.GetActorForwardVector`) 1000.0) true))))
    (:`NewEnumerator1`
      (goto _label_2))
    (:`NewEnumerator2`
      (set `self.SwordState` "NewEnumerator7" :!label _label_4)
      ;[1 1 1] AirAttack
      (switch `int` _attackcount :!label _label_5
        (:`0`
          (set `self.AttackCount` 1)
          (`self.PlayAnimMontage` "/Game/Animation/JumpCombo3_1.JumpCombo3_1"))
        (:`1`
          (set `self.AttackCount` 2)
          (`self.PlayAnimMontage` "/Game/Animation/JumpCombo3_2.JumpCombo3_2"))
        (:`2`
          (set `self.AttackCount` 0)
          (`self.PlayAnimMontage` "/Game/Animation/JumpCombo3_3.JumpCombo3_3")))
      (`self.LaunchCharacter` (0.0 0.0 500.0) false true))
    (:`NewEnumerator3`
      (goto _label_4))
    (:`NewEnumerator6`
      (set `self.SaveAttack` true :!label _label_6))
    (:`NewEnumerator7`
      (goto _label_6))))

(event `ComboAttackSave`
  ;[1 1 1] SetCombo
  (if (`self.SaveAttack`)
    (set `self.SaveAttack` false)
    (switch `/Game/Enum/EnumSwordState` (`self.SwordState`)
      (:`NewEnumerator6`
        (goto _label_3))
      (:`NewEnumerator7`
        (goto _label_5)))))

(event `DodgeEvent`
  (params (Dir :type "Vector Structure"))
  (bind _returnvalue (+ (* Dir_X (`self.GetActorForwardVector`)) (* Dir_Y (`self.GetActorRightVector`))))
  (bind _returnvalue_2 (`KismetAnimationLibrary.CalculateDirection` _returnvalue (`self.K2_GetActorRotation`)))
  ;[1 1 1] Dodge
  (switch `/Game/Enum/EnumSwordState` (`self.SwordState`)
    (:`NewEnumerator0`
      _)
    (:`NewEnumerator1`
      _)
    (:`NewEnumerator6`
      _))
  (set `self.SwordState` "NewEnumerator5")
  (if (< (`KismetMathLibrary.Abs` _returnvalue_2) 45.0)
    (`self.PlayAnimMontage` "/Game/Animation/DodgeForward.DodgeForward")
    (elif (> (`KismetMathLibrary.Abs` _returnvalue_2) 135.0)
      (`self.PlayAnimMontage` "/Game/Animation/DodgeBack.DodgeBack")
      (elif (> _returnvalue_2 0.0)
        (`self.PlayAnimMontage` "/Game/Animation/DodgeRight.DodgeRight")
        (else
          (`self.PlayAnimMontage` "/Game/Animation/DodgeLeft.DodgeLeft")))))
  (`self.LaunchCharacter` (* (`KismetMathLibrary.Vector_NormalUnsafe` _returnvalue) 1500.0) true))

(event `EndDodge`
  ;[1 1 1] EndDodge
  (set `self.SwordState` "NewEnumerator0")
  (set `MovementComponent.Velocity` (0.0 0.0 0.0) (`self.CharacterMovement`))
  (cast `/Game/BP/BP_PlayerController` (`self.GetController`)))

(event `ResetCombo`
  ;[1 1 1] ResetCombo
  (set `self.AttackCount` 0)
  (set `self.SaveAttack` false)
  (set `self.IsAttacking` false)
  (switch `/Game/Enum/EnumSwordState` (`self.SwordState`)
    (:`NewEnumerator6`
      (set `self.SwordState` "NewEnumerator0"))
    (:`NewEnumerator7`
      (set `self.SwordState` "NewEnumerator4"))))

(fn `UserConstructionScript`)