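; Player controller that turns Enhanced Input into movement, camera rotation, jump, attack and dodge for BP_Player.
; Each tick it caches the pawn's SwordState, which gates movement input.
; Most states ease the pawn toward control yaw and move it camera-relative, while Dodge and Ground Attack only turn it and record DodgeDir.
; Jump, attack and dodge inputs forward to BP_Player events, with dodge passing that direction.
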(event `self.ReceiveBeginPlay`
  (`EnhancedInputSubsystemInterface.AddMappingContext` (subsystem `EnhancedInputLocalPlayerSubsystem`) "/Game/MyContents/BP/IMC_Player.IMC_Player" 0 (struct)))

(event `self.ReceiveTick`
  (params (DeltaSeconds :type "Float (single-precision)"))
  (bind _asbp_player (cast `/Game/MyContents/BP/BP_Player` (`self.K2_GetPawn`)))
  (set `self.SwordState` (`/Game/MyContents/BP/BP_Player.SwordState` _asbp_player)))

(event `SetMovement`
  (params (CanMove :type Boolean))
  (set `self.CanMove` CanMove))

(event `EnhancedInput|/Game/MyContents/BP/IA_Movement`
  (params (ActionValue :type "Vector2D Structure") (ElapsedSeconds :type "Float (double-precision)") (TriggeredSeconds :type "Float (double-precision)") (InputAction :type "InputAction Object Reference" :default "/Game/MyContents/BP/IA_Movement.IA_Movement"))
  (bind _returnvalue (`self.K2_GetPawn`))
  (bind (_returnvalue_roll _returnvalue_pitch _returnvalue_yaw) (`KismetMathLibrary.BreakRotator` (`self.GetControlRotation`)))
  (bind _returnvalue_2 (`KismetMathLibrary.GetForwardVector` (`KismetMathLibrary.MakeRotator` 0.0 0.0 _returnvalue_yaw)))
  (bind _returnvalue_3 (`KismetMathLibrary.RLerp` (`KismetMathLibrary.Conv_VectorToRotator` (`self.GetActorForwardVector` _returnvalue)) (`KismetMathLibrary.Conv_VectorToRotator` _returnvalue_2) 0.05 true))
  ;[0 0.3826 1] Movement
  (:`Triggered`
    (switch `/Game/MyContents/Enum/EnumSwordState` (`self.SwordState`)
      (:`NewEnumerator0`
        (`self.K2_SetActorRotation` _returnvalue _returnvalue_3 false :!label _label)
        (`Pawn.AddMovementInput` _returnvalue _returnvalue_2 ActionValue_X false)
        (`Pawn.AddMovementInput` _returnvalue (`KismetMathLibrary.GetRightVector` (`KismetMathLibrary.MakeRotator` 0.0 0.0 _returnvalue_yaw)) ActionValue_Y false))
      (:`NewEnumerator1`
        (goto _label))
      (:`NewEnumerator2`
        (goto _label))
      (:`NewEnumerator3`
        (goto _label))
      (:`NewEnumerator4`
        (goto _label))
      (:`NewEnumerator5`
        (set `self.DodgeDir` (`KismetMathLibrary.MakeVector` ActionValue_X ActionValue_Y) :!label _label_2)
        (`self.K2_SetActorRotation` _returnvalue _returnvalue_3 false))
      (:`NewEnumerator6`
        (goto _label_2))
      (:`NewEnumerator7`
        (goto _label)))))

(event `EnhancedInput|/Game/MyContents/BP/IA_Rotate`
  (params (ActionValue :type "Vector2D Structure") (ElapsedSeconds :type "Float (double-precision)") (TriggeredSeconds :type "Float (double-precision)") (InputAction :type "InputAction Object Reference" :default "/Game/MyContents/BP/IA_Rotate.IA_Rotate"))
  ;[0 0.1803 0.4072] Rotate
  (:`Triggered`
    (`self.AddYawInput` ActionValue_X)
    (`self.AddPitchInput` ActionValue_Y)))

(event `EnhancedInput|/Game/MyContents/BP/IA_Jump`
  (params (ActionValue :type Boolean) (ElapsedSeconds :type "Float (double-precision)") (TriggeredSeconds :type "Float (double-precision)") (InputAction :type "InputAction Object Reference" :default "/Game/MyContents/BP/IA_Jump.IA_Jump"))
  ;[0.0349 0.4746 1] Jump/DoubleJump
  (:`Started`
    (bind _asbp_player (cast `/Game/MyContents/BP/BP_Player` (`self.K2_GetPawn`)))
    (`/Game/MyContents/BP/BP_Player.JumpEvent` _asbp_player)))

(event `EnhancedInput|/Game/MyContents/BP/IA_Attack`
  (params (ActionValue :type Boolean) (ElapsedSeconds :type "Float (double-precision)") (TriggeredSeconds :type "Float (double-precision)") (InputAction :type "InputAction Object Reference" :default "/Game/MyContents/BP/IA_Attack.IA_Attack"))
  ;[1 0.01884 0.07856] LandCombo3
  (:`Started`
    (bind _asbp_player (cast `/Game/MyContents/BP/BP_Player` (`self.K2_GetPawn`)))
    (`/Game/MyContents/BP/BP_Player.Combo3Input` _asbp_player)))

(event `EnhancedInput|/Game/MyContents/BP/IA_Dodge`
  (params (ActionValue :type Boolean) (ElapsedSeconds :type "Float (double-precision)") (TriggeredSeconds :type "Float (double-precision)") (InputAction :type "InputAction Object Reference" :default "/Game/MyContents/BP/IA_Dodge.IA_Dodge"))
  (bind (_dodgedir_x _dodgedir_y) (`KismetMathLibrary.BreakVector` (`self.DodgeDir`)))
  ;[1 1 1] Dodge
  (:`Triggered`
    (bind _asbp_player (cast `/Game/MyContents/BP/BP_Player` (`self.K2_GetPawn`)))
    (`/Game/MyContents/BP/BP_Player.DodgeEvent` _asbp_player (`KismetMathLibrary.MakeVector` _dodgedir_x _dodgedir_y))))

(fn `UserConstructionScript`)