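; BP_EnemySpawner is an actor that periodically spawns BP_Enemy1 enemies around itself.
; Tick accumulates delta time in a timer and, every few seconds, resets it and spawns one enemy.
; Each spawn lands at a random X and Y offset within a wide square centered on the spawner, at the spawner's own height.
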(event `self.ReceiveBeginPlay`)

(event `self.ReceiveTick`
  (params (DeltaSeconds :type "Float (single-precision)"))
  (bind (_returnvalue_x _returnvalue_y _returnvalue_z) (`KismetMathLibrary.BreakVector` (`self.K2_GetActorLocation`)))
  (bind _output_get (set `self.Timer` (+ DeltaSeconds (`self.Timer`))))
  (if (> _output_get 3.0)
    (set `self.Timer` 0.0)
    (`|SpawnActorFromClass` "/Game/MyContents/BP/BP_Enemy1.BP_Enemy1_C" (`KismetMathLibrary.MakeTransform` (`KismetMathLibrary.MakeVector` (+ (`KismetMathLibrary.RandomFloatInRange` -3000.0 3000.0) _returnvalue_x) (+ _returnvalue_y (`KismetMathLibrary.RandomFloatInRange` -3000.0 3000.0)) _returnvalue_z)) "Undefined" "MultiplyWithRoot" null null)))

(fn `UserConstructionScript`)