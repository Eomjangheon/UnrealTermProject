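; BP_Proj is a sword slash projectile that damages BP_Enemy1 actors.
; On BeginPlay it sets its projectile velocity from Dir and Speed, reveals one of two slash components chosen by Index, then destroys itself after Time seconds.
; Box overlaps with that exact enemy class apply Damage and spawn a shockwave effect and impact sound, without destroying the projectile on hit.
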(event `self.ReceiveBeginPlay`
  (set `MovementComponent.Velocity` (* (`self.Dir`) (`self.Speed`)) (`self.ProjectileMovement`))
  (switch `int` (`self.Index`)
    (:`0`
      (`SceneComponent.SetVisibility` (`self.Slash_0`) true false))
    (:`1`
      (`SceneComponent.SetVisibility` (`self.Slash_1`) true false)))
  (`KismetSystemLibrary.Delay` (`self.Time`))
  (`self.K2_DestroyActor`))

(event `self.Box.OnComponentBeginOverlap`
  (params (OverlappedComponent :type "PrimitiveComponent Object Reference") (OtherActor :type "Actor Object Reference") (OtherComp :type "PrimitiveComponent Object Reference") (OtherBodyIndex :type Integer) (bFromSweep :type Boolean) (SweepResult :type "HitResult Structure (by ref)"))
  (bind _returnvalue (`SceneComponent.K2_GetComponentLocation` (`self.Box`)))
  (if (== (`GameplayStatics.GetObjectClass` OtherActor) "/Game/MyContents/BP/BP_Enemy1.BP_Enemy1_C")
    (`GameplayStatics.ApplyDamage` OtherActor (`self.Damage`) null self)
    (`GameplayStatics.SpawnEmitterAtLocation` "/Game/FXVarietyPack/Particles/P_ky_shotShockwave.P_ky_shotShockwave" _returnvalue (`KismetMathLibrary.FindLookAtRotation` _returnvalue (`self.K2_GetActorLocation`)))
    (`GameplayStatics.PlaySoundAtLocation` "/Game/MyContents/Sounds/SwordSFX/SWSH_Sword_Slash_Impact_V2_Assorted_18_DDUMAIS_NONE.SWSH_Sword_Slash_Impact_V2_Assorted_18_DDUMAIS_NONE" _returnvalue (struct) 1.0 1.0 0.0 null null null null)))

(fn `UserConstructionScript`)