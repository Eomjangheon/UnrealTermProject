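; BP_DamageInd is a short-lived floating damage indicator actor that shows a damage amount and whether the hit is critical.
; On BeginPlay it passes both values to its widget through an interface call.
; It picks a randomized end point offset up and right, using vectors fetched from player character 0 through an interface.
; A Timeline lerps the actor to that point, then destroys it when finished.
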(event `self.ReceiveBeginPlay`
  (message `/Game/MyContents/UI/BPI_DamageInd.IF_SetDamage` (`WidgetComponent.GetWidget` (`self.DamageWidget`)) (`self.Damage`) (`self.IsCritical`))
  (bind _output_get (set `self.StartPos` (`self.K2_GetActorLocation`)))
  (bind (_upvector _rightvector) (message `/Game/MyContents/UI/BPI_DamageGiverInd.IF_GetVectors` (`GameplayStatics.GetPlayerCharacter` 0)))
  (set `self.EndPos` (+ _output_get (* _upvector (`KismetMathLibrary.RandomFloatInRange` 40.0 50.0)) (* _rightvector (`KismetMathLibrary.RandomFloatInRange` 20.0 30.0))))
  (bind (_direction _newtrack_0) (`Timeline|Timeline`)
    (:`Update`
      (`self.K2_SetActorLocation` (`KismetMathLibrary.VLerp` (`self.StartPos`) (`self.EndPos`) _newtrack_0)))
    (:`Finished`
      (`self.K2_DestroyActor`))))

(fn `UserConstructionScript`)